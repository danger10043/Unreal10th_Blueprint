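; BP_Day0617_P1_2 is an actor that shuttles back and forth along its forward vector from its starting location.
; BeginPlay caches that location, and Tick accumulates delta time in a repeating six-second cycle.
; Each frame sets position from elapsed time and MoveSpeed without sweep: outward for three seconds, then back for three.
; On the frame the timer wraps, it skips the position update.
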(event `self.ReceiveBeginPlay`
  (set `self.ActorInitialLocation` (`self.K2_GetActorLocation`)))

(event `self.ReceiveTick`
  (params (DeltaSeconds :type "Float (single-precision)"))
  (bind _output_get (set `self.TimeSum` (+ DeltaSeconds (`self.TimeSum`))))
  (if (<= _output_get 3.0)
    (`self.K2_SetActorLocation` (+ (* (`self.GetActorForwardVector`) (`self.MoveSpeed`) (`self.TimeSum`)) (`self.ActorInitialLocation`)))
    (elif (>= (`self.TimeSum`) 6.0)
      (set `self.TimeSum` (- (`self.TimeSum`) 6.0))
      (else
        (`self.K2_SetActorLocation` (+ (* (`self.GetActorForwardVector`) (`self.MoveSpeed`) (- 6.0 (`self.TimeSum`))) (`self.ActorInitialLocation`)))))))

(fn `UserConstructionScript`)