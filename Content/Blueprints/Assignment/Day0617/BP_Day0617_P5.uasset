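; Double sliding door actor that animates its two panels as soon as play begins.
; BeginPlay caches each door's relative location, then plays a timeline.
; The timeline's DoorMovement track is scaled into a Y offset, moving the left and right doors in opposite directions from their starting positions.
; Overlap and Tick events are unused, so the movement has no player trigger.
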(event `self.ReceiveBeginPlay`
  (bind (_leftdoorinitiallocation_x _leftdoorinitiallocation_y _leftdoorinitiallocation_z) (`KismetMathLibrary.BreakVector` (`self.LeftDoorInitialLocation`)))
  (bind (_rightdoorinitiallocation_x _rightdoorinitiallocation_y _rightdoorinitiallocation_z) (`KismetMathLibrary.BreakVector` (`self.RightDoorInitialLocation`)))
  (set `self.LeftDoorInitialLocation` (`SceneComponent.RelativeLocation` (`self.LeftDoor`)))
  (set `self.RightDoorInitialLocation` (`SceneComponent.RelativeLocation` (`self.RightDoor`)))
  (bind (_direction _doormovement) (`Timeline|타임라인`)
    (:`Update`
      (bind _returnvalue (* _doormovement 85.0))
      (`SceneComponent.K2_SetRelativeLocation` (`self.LeftDoor`) (`KismetMathLibrary.MakeVector` _leftdoorinitiallocation_x (+ _leftdoorinitiallocation_y _returnvalue) _leftdoorinitiallocation_z) false false)
      (`SceneComponent.K2_SetRelativeLocation` (`self.RightDoor`) (`KismetMathLibrary.MakeVector` _rightdoorinitiallocation_x (+ _rightdoorinitiallocation_y (* -1.0 _returnvalue)) _rightdoorinitiallocation_z) false false))))

(fn `UserConstructionScript`)