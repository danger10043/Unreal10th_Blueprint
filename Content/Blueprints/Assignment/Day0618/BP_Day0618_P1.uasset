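; BP_Day0618_P1 is an actor that moves back and forth along its forward vector.
; Tick accumulates elapsed time and uses its sine as a velocity, with MovePhase as peak speed and MovePeriod as angular frequency.
; Each frame adds that delta-scaled step to the current location without sweeping, so the motion is integrated rather than computed from a stored origin.
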(event `self.ReceiveBeginPlay`
  (set `self.ElpasedTime` 0.0))

(event `self.ReceiveTick`
  (params (DeltaSeconds :type "Float (single-precision)"))
  (bind _output_get (set `self.ElpasedTime` (+ DeltaSeconds (`self.ElpasedTime`))))
  (`self.K2_SetActorLocation` (+ (`self.K2_GetActorLocation`) (* (`self.GetActorForwardVector`) (`self.MovePhase`) DeltaSeconds (`KismetMathLibrary.Sin` (* _output_get (`self.MovePeriod`)))))))

(fn `UserConstructionScript`)