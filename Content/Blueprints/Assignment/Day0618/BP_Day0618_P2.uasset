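; BP_Day0618_P2 is a plane actor that homes in on the player and knocks them away on contact.
; Each Tick it eases its rotation toward the player pawn with RInterpTo, moves along its forward vector by MoveSpeed and rolls PlanePropeller by RotateSpeed.
; Movement and spin are per-frame steps, unscaled by delta time and without sweep.
; Hitting the player applies a large velocity-change impulse opposite the hit normal through BP_Day0622_Player's CharacterMovement.
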(event `self.ReceiveTick`
  (params (DeltaSeconds :type "Float (single-precision)"))
  (bind _returnvalue (`self.K2_GetActorLocation`))
  (bind _planepropeller (`self.PlanePropeller`))
  (bind (_relativerotation_roll _relativerotation_pitch _relativerotation_yaw) (`KismetMathLibrary.BreakRotator` (`SceneComponent.RelativeRotation` _planepropeller)))
  (bind _output_get (set `self.TargetLocation` (`self.K2_GetActorLocation` (`GameplayStatics.GetPlayerPawn` 0))))
  (set `self.TargetDirection` (`KismetMathLibrary.Normal` (- _output_get _returnvalue)))
  (`self.K2_SetActorRotation` (`KismetMathLibrary.RInterpTo` (`self.K2_GetActorRotation`) (`KismetMathLibrary.Conv_VectorToRotator` (`self.TargetDirection`)) DeltaSeconds 0.99))
  (`self.K2_SetActorLocation` (+ (* (`self.GetActorForwardVector`) (`self.MoveSpeed`)) (+ (0.0 0.0 0.0) _returnvalue)))
  (`SceneComponent.K2_SetRelativeRotation` _planepropeller (`KismetMathLibrary.MakeRotator` (+ (`self.RotateSpeed`) _relativerotation_roll) _relativerotation_pitch _relativerotation_yaw) false false))

(event `self.ReceiveHit`
  (params (MyComp :type "PrimitiveComponent Object Reference") (Other :type "Actor Object Reference") (OtherComp :type "PrimitiveComponent Object Reference") (bSelfMoved :type Boolean) (HitLocation :type "Vector Structure") (HitNormal :type "Vector Structure") (NormalImpulse :type "Vector Structure") (Hit :type "HitResult Structure (by ref)"))
  (bind _returnvalue (`GameplayStatics.GetPlayerPawn` 0))
  (if (== Other _returnvalue)
    (bind _asbp_day_0622_player (cast `/Game/Blueprints/Assignment/Day0622/BP_Day0622_Player` _returnvalue))
    (`CharacterMovementComponent.AddImpulse` (`Character.CharacterMovement` _asbp_day_0622_player) (* HitNormal -15000.0) true)))

(fn `UserConstructionScript`)