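; An actor that rises and travels horizontally while the player pawn overlaps it, like a player-steered hover platform.
; A timeline's height alpha, scaled by FloatHeight, offsets its Z from the BeginPlay location and reverses when the overlap ends.
; Overlap sets CurrentVelocity to Velocity and end overlap zeroes it.
; Tick moves the actor by that speed along the player pawn's forward vector, without sweep.
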(event `self.ReceiveBeginPlay`
  (set `self.InitialLocation` (`self.K2_GetActorLocation`)))

(event `self.ReceiveActorBeginOverlap`
  (params (OtherActor :type "Actor Object Reference"))
  (bind (_returnvalue_x _returnvalue_y) (`KismetMathLibrary.BreakVector` (`self.K2_GetActorLocation`)))
  (bind (_initiallocation_x _initiallocation_y _initiallocation_z) (`KismetMathLibrary.BreakVector` (`self.InitialLocation`)))
  (if (== OtherActor (`GameplayStatics.GetPlayerPawn` 0))
    (set `self.CurrentVelocity` (`self.Velocity`))
    (bind (_direction _heightalpha) (`Timeline|타임라인` :!label _label)
      (:`Update`
        (`self.K2_SetActorLocation` (`KismetMathLibrary.MakeVector` _returnvalue_x _returnvalue_y (+ (* _heightalpha (`self.FloatHeight`)) _initiallocation_z)))))))

(event `self.ReceiveActorEndOverlap`
  (params (OtherActor :type "Actor Object Reference"))
  (if (== OtherActor (`GameplayStatics.GetPlayerPawn` 0))
    (set `self.CurrentVelocity` 0.0)
    (goto _label :!via `Reverse`)))

(event `self.ReceiveTick`
  (params (DeltaSeconds :type "Float (single-precision)"))
  (`self.K2_SetActorLocation` (+ (* (`self.GetActorForwardVector` (`GameplayStatics.GetPlayerPawn` 0)) DeltaSeconds (`self.CurrentVelocity`)) (`self.K2_GetActorLocation`))))

(fn `UserConstructionScript`)