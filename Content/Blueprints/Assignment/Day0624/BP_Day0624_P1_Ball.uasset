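; Ball Blueprint for a Day0624 assignment that fades a lamp's color on the BP_Day0624_P1 actor.
; TurnonLamp and TurnOffLamp each look up that actor by class and check that it is valid.
; Each drives its own Timeline, played forward for on and in reverse for off, feeding ColorAlpha into the green channel of LampColor's "Color" parameter.
; No caller for either event appears here.
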(event `/Game/Blueprints/Assignment/Day0624/BPI_Day0624_P1.TurnOnLamp`
  (bind _returnvalue (`GameplayStatics.GetActorOfClass` "/Game/Blueprints/Assignment/Day0624/BP_Day0624_P1.BP_Day0624_P1_C"))
  (`/Engine/EditorBlueprintResources/StandardMacros.IsValid` _returnvalue
    (:`Is Valid`
      (bind (_direction _coloralpha) (`Timeline|타임라인` :!via `PlayFromStart`)
        (:`Update`
          (`MaterialInstanceDynamic.SetVectorParameterValue` (`/Game/Blueprints/Assignment/Day0624/BP_Day0624_P1.LampColor` _returnvalue) "Color" (make `LinearColor` 0.0 _coloralpha 0.0 1.0)))))))

(event `/Game/Blueprints/Assignment/Day0624/BPI_Day0624_P1.TurnOffLamp`
  (bind _returnvalue (`GameplayStatics.GetActorOfClass` "/Game/Blueprints/Assignment/Day0624/BP_Day0624_P1.BP_Day0624_P1_C"))
  (`/Engine/EditorBlueprintResources/StandardMacros.IsValid` _returnvalue
    (:`Is Valid`
      (bind (_direction _coloralpha) (`Timeline|타임라인_0` :!via `ReverseFromEnd`)
        (:`Update`
          (`MaterialInstanceDynamic.SetVectorParameterValue` (`/Game/Blueprints/Assignment/Day0624/BP_Day0624_P1.LampColor` _returnvalue) "Color" (make `LinearColor` 0.0 _coloralpha 0.0 1.0)))))))

(fn `UserConstructionScript`)