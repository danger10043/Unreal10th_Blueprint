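; A sliding double door with a push button, whose open, close, toggle and press events are not called within this Blueprint.
; Open and Close flip the Opened flag and play one timeline forward or in reverse, sliding both doors apart or together from cached positions.
; Separate timelines move the button along X and drive the red GlowColor of its dynamic material.
; Overlap events track whether the player pawn is in front through IsPlayerFront.
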(event `self.ReceiveBeginPlay`
  (bind _button (`self.Button`))
  (set `self.LeftDoorInitialLocation` (`SceneComponent.RelativeLocation` (`self.LeftDoor`)))
  (set `self.RightDoorInitialLocation` (`SceneComponent.RelativeLocation` (`self.RightDoor`)))
  (set `self.ButtonInitialLocation` (`SceneComponent.RelativeLocation` _button))
  (bind _returnvalue (`PrimitiveComponent.CreateDynamicMaterialInstance` _button 0 (`PrimitiveComponent.GetMaterial` _button 0) "None"))
  (set `self.ButtonColor` _returnvalue))

(event `Open`
  (bind (_leftdoorinitiallocation_x _leftdoorinitiallocation_y _leftdoorinitiallocation_z) (`KismetMathLibrary.BreakVector` (`self.LeftDoorInitialLocation`)))
  (bind (_rightdoorinitiallocation_x _rightdoorinitiallocation_y _rightdoorinitiallocation_z) (`KismetMathLibrary.BreakVector` (`self.RightDoorInitialLocation`)))
  (`self.SwitchBOpened` :!label _label)
  (bind (_direction _doormovement) (`Timeline|타임라인` :!via `PlayFromStart` :!label _label_2)
    (:`Update`
      (bind _returnvalue (* _doormovement 85.0))
      (`SceneComponent.K2_SetRelativeLocation` (`self.LeftDoor`) (`KismetMathLibrary.MakeVector` _leftdoorinitiallocation_x (+ _leftdoorinitiallocation_y _returnvalue) _leftdoorinitiallocation_z) false false)
      (`SceneComponent.K2_SetRelativeLocation` (`self.RightDoor`) (`KismetMathLibrary.MakeVector` _rightdoorinitiallocation_x (+ _rightdoorinitiallocation_y (* -1.0 _returnvalue)) _rightdoorinitiallocation_z) false false))))

(event `Close`
  (`self.SwitchBOpened` :!label _label_3)
  (goto _label_2 :!via `ReverseFromEnd`))

(event `Switch Open State`
  (if (`self.bOpened`)
    (goto _label_3)
    (else
      (goto _label))))

(event `Press Button`
  (bind (_buttoninitiallocation_x _buttoninitiallocation_y _buttoninitiallocation_z) (`KismetMathLibrary.BreakVector` (`self.ButtonInitialLocation`)))
  (bind (_direction `_새_트랙_0`) (`Timeline|타임라인_0` :!via `PlayFromStart`)
    (:`Update`
      (`SceneComponent.K2_SetRelativeLocation` (`self.Button`) (`KismetMathLibrary.MakeVector` (+ `_새_트랙_0` _buttoninitiallocation_x) _buttoninitiallocation_y _buttoninitiallocation_z) false false))))

(event `Press Button Light`
  (bind (_direction _buttoncolorvalue) (`Timeline|타임라인_1` :!via `PlayFromStart`)
    (:`Update`
      (`MaterialInstanceDynamic.SetVectorParameterValue` (`self.ButtonColor`) "GlowColor" (make `LinearColor` _buttoncolorvalue 0.0 0.0 1.0)))))

(event `self.ReceiveActorBeginOverlap`
  (params (OtherActor :type "Actor Object Reference"))
  (if (== OtherActor (`GameplayStatics.GetPlayerPawn` 0))
    (set `self.bIsPlayerFront` true)))

(event `self.ReceiveActorEndOverlap`
  (params (OtherActor :type "Actor Object Reference"))
  (if (== OtherActor (`GameplayStatics.GetPlayerPawn` 0))
    (set `self.bIsPlayerFront` false)))

(fn `SwitchBOpened`
  (set `self.bOpened` (not (`self.bOpened`)))
  (return))

(fn `UserConstructionScript`)