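; Base jetpack actor that lifts the Character owning it as parent actor and runs on limited energy.
; Activate and deactivate events toggle the two exhaust effects and swap the character's air control.
; While active, Tick drains energy by elapsed time, calls LaunchCharacter upward every frame and shuts off when empty.
; Dynamic materials show the pack color and an energy glow that dims with the fourth power of remaining charge.
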(event `self.ReceiveBeginPlay`
  (bind _backpackright (`self.BackpackRight`))
  (bind _backpackleft (`self.BackpackLeft`))
  (bind _backpackenergyviewer (`self.BackpackEnergyViewer`))
  (bind `_as캐릭터` (cast `Character` (`self.GetParentActor`)))
  (set `self.ParentCharacter` `_as캐릭터`)
  (bind _returnvalue (`PrimitiveComponent.CreateDynamicMaterialInstance` _backpackright 0 (`PrimitiveComponent.GetMaterial` _backpackright 0) "None"))
  (set `self.JetpackRightColorMID` _returnvalue)
  (bind _returnvalue_2 (`PrimitiveComponent.CreateDynamicMaterialInstance` _backpackleft 0 (`PrimitiveComponent.GetMaterial` _backpackleft 0) "None"))
  (set `self.JetpackLeftColorMID` _returnvalue_2)
  (bind _returnvalue_3 (`PrimitiveComponent.CreateDynamicMaterialInstance` _backpackenergyviewer 0 (`PrimitiveComponent.GetMaterial` _backpackenergyviewer 0) "None"))
  (set `self.JetpackEnergyViewerColorMID` _returnvalue_3))

(event `/Game/Blueprints/Assignment/Day0625/FrameWorks/BPI_Day0625_Jetpack.ActivateJetpack`
  (bind _parentcharacter (`self.ParentCharacter`))
  (`/Engine/EditorBlueprintResources/StandardMacros.IsValid` _parentcharacter
    (:`Is Valid`
      (set `self.bActivatedJetpack` true)
      (set `CharacterMovementComponent.AirControl` (`self.HoverSpeed`) (`Character.CharacterMovement` _parentcharacter))
      (`ActorComponent.Activate` (`self.BackpackEffectLeft`) false)
      (`ActorComponent.Activate` (`self.BackpackEffectRight`) false))))

(event `/Game/Blueprints/Assignment/Day0625/FrameWorks/BPI_Day0625_Jetpack.DeactivateJetpack`
  (bind _parentcharacter (`self.ParentCharacter`))
  (`/Engine/EditorBlueprintResources/StandardMacros.IsValid` _parentcharacter
    (:`Is Valid`
      (set `self.bActivatedJetpack` false)
      (set `CharacterMovementComponent.AirControl` (`self.InitialHoverSpeed`) (`Character.CharacterMovement` _parentcharacter))
      (`ActorComponent.Deactivate` (`self.BackpackEffectLeft`))
      (`ActorComponent.Deactivate` (`self.BackpackEffectRight`)))))

(event `self.ReceiveTick`
  (params (DeltaSeconds :type "Float (single-precision)"))
  (bind (_returnvalue_r _returnvalue_g _returnvalue_b) (break `LinearColor` (`KismetMathLibrary.Conv_ColorToLinearColor` (`self.JetpackEnergyColor`))))
  (bind _returnvalue (* (`KismetMathLibrary.Square` (`KismetMathLibrary.Square` (/ (`KismetMathLibrary.FMax` (`self.CurrentEnergy`)) (`self.MaxEnergy`)))) 10.0))
  (`MaterialInstanceDynamic.SetVectorParameterValue` (`self.JetpackRightColorMID`) "MainColor" (`KismetMathLibrary.Conv_ColorToLinearColor` (`self.JetpackColor`)))
  (`MaterialInstanceDynamic.SetVectorParameterValue` (`self.JetpackLeftColorMID`) "MainColor" (`KismetMathLibrary.Conv_ColorToLinearColor` (`self.JetpackColor`)))
  (`MaterialInstanceDynamic.SetVectorParameterValue` (`self.JetpackEnergyViewerColorMID`) "EnergyColor" (make `LinearColor` (* _returnvalue_r _returnvalue) (* _returnvalue_g _returnvalue) (* _returnvalue_b _returnvalue) 1.0))
  (if (and (`self.bActivatedJetpack`) (>= (`self.CurrentEnergy`) 0.0))
    (bind _output_get (set `self.CurrentEnergy` (- (`self.CurrentEnergy`) DeltaSeconds)))
    (if (<= _output_get 0.0)
      (`self.DeactivateJetpack`)))
  (if (`self.bActivatedJetpack`)
    (`Character.LaunchCharacter` (`self.ParentCharacter`) (`KismetMathLibrary.MakeVector` 0.0 0.0 (`self.ThrustPower`)) false false)))

(fn `UserConstructionScript`)