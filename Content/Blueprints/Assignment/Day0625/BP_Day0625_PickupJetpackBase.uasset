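; A jetpack pickup that floats with a sine bob, spins, and equips a jetpack on the player on overlap.
; BeginPlay creates dynamic materials on the backpack meshes to show the pickup's body and energy colors.
; On overlap, if the player's backpack child actor is empty, it spawns a BP_Day0625_JetPackBase there, copies its colors, hover, thrust and full energy across, then destroys itself.
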(event `self.ReceiveBeginPlay`
  (bind _backpackright (`self.BackpackRight`))
  (bind _backpackleft (`self.BackpackLeft`))
  (bind _backpackenergyviewer (`self.BackpackEnergyViewer`))
  (set `self.ParentCharacter` null)
  (bind _returnvalue (`PrimitiveComponent.CreateDynamicMaterialInstance` _backpackright 0 (`PrimitiveComponent.GetMaterial` _backpackright 0) "None"))
  (set `self.JetpackRightColorMID` _returnvalue)
  (bind _returnvalue_2 (`PrimitiveComponent.CreateDynamicMaterialInstance` _backpackleft 0 (`PrimitiveComponent.GetMaterial` _backpackleft 0) "None"))
  (set `self.JetpackLeftColorMID` _returnvalue_2)
  (bind _returnvalue_3 (`PrimitiveComponent.CreateDynamicMaterialInstance` _backpackenergyviewer 0 (`PrimitiveComponent.GetMaterial` _backpackenergyviewer 0) "None"))
  (set `self.JetpackEnergyViewerColorMID` _returnvalue_3)
  (set `self.InitialLocation` (`self.K2_GetActorLocation`))
  (`MaterialInstanceDynamic.SetVectorParameterValue` (`self.JetpackRightColorMID`) "MainColor" (`KismetMathLibrary.Conv_ColorToLinearColor` (`self.JetpackColor`)))
  (`MaterialInstanceDynamic.SetVectorParameterValue` (`self.JetpackLeftColorMID`) "MainColor" (`KismetMathLibrary.Conv_ColorToLinearColor` (`self.JetpackColor`)))
  (`MaterialInstanceDynamic.SetVectorParameterValue` (`self.JetpackEnergyViewerColorMID`) "EnergyColor" (`KismetMathLibrary.Conv_ColorToLinearColor` (`self.JetpackEnergyColor`))))

(event `self.ReceiveActorBeginOverlap`
  (params (OtherActor :type "Actor Object Reference"))
  (bind _returnvalue (`GameplayStatics.GetPlayerPawn` 0))
  (if (== OtherActor _returnvalue)
    (bind _asbp_day_0625_player (cast `/Game/Blueprints/Assignment/Day0625/BP_Day0625_Player` _returnvalue))
    (bind _backpackchildactor (`/Game/Blueprints/Assignment/Day0625/BP_Day0625_Player.BackpackChildActor` _asbp_day_0625_player))
    (bind _childactor (`ChildActorComponent.ChildActor` _backpackchildactor))
    (`/Engine/EditorBlueprintResources/StandardMacros.IsValid` _childactor
      (:`Is Not Valid`
        (`ChildActorComponent.SetChildActorClass` _backpackchildactor "/Game/Blueprints/Assignment/Day0625/BP_Day0625_JetPackBase.BP_Day0625_JetPackBase_C")
        (bind _asbp_day_0625_jet_pack_base (cast `/Game/Blueprints/Assignment/Day0625/BP_Day0625_JetPackBase` _childactor))
        (set `/Game/Blueprints/Assignment/Day0625/BP_Day0625_JetPackBase.HoverSpeed` (`self.HoverSpeed`) _asbp_day_0625_jet_pack_base)
        (set `/Game/Blueprints/Assignment/Day0625/BP_Day0625_JetPackBase.JetpackColor` (`self.JetpackColor`) _asbp_day_0625_jet_pack_base)
        (set `/Game/Blueprints/Assignment/Day0625/BP_Day0625_JetPackBase.JetpackEnergyColor` (`self.JetpackEnergyColor`) _asbp_day_0625_jet_pack_base)
        (set `/Game/Blueprints/Assignment/Day0625/BP_Day0625_JetPackBase.ThrustPower` (`self.ThrustPower`) _asbp_day_0625_jet_pack_base)
        (set `/Game/Blueprints/Assignment/Day0625/BP_Day0625_JetPackBase.MaxEnergy` (`self.MaxEnergy`) _asbp_day_0625_jet_pack_base)
        (set `/Game/Blueprints/Assignment/Day0625/BP_Day0625_JetPackBase.CurrentEnergy` (`self.MaxEnergy`) _asbp_day_0625_jet_pack_base)
        (`self.K2_DestroyActor`)))))

(event `self.ReceiveTick`
  (params (DeltaSeconds :type "Float (single-precision)"))
  (bind (_returnvalue_roll _returnvalue_pitch _returnvalue_yaw) (`KismetMathLibrary.BreakRotator` (`self.K2_GetActorRotation`)))
  (bind (_initiallocation_x _initiallocation_y _initiallocation_z) (`KismetMathLibrary.BreakVector` (`self.InitialLocation`)))
  (bind _output_get (set `self.TimeElapsed` (+ DeltaSeconds (`self.TimeElapsed`))))
  (`self.K2_SetActorLocation` (`KismetMathLibrary.MakeVector` _initiallocation_x _initiallocation_y (+ _initiallocation_z (* (`KismetMathLibrary.Sin` _output_get) 25.0))))
  (`self.K2_SetActorRotation` (`KismetMathLibrary.MakeRotator` _returnvalue_roll _returnvalue_pitch (+ (* DeltaSeconds 50.0) _returnvalue_yaw))))

(fn `UserConstructionScript`)