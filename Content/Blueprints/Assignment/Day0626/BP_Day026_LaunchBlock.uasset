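; BP_Day026_LaunchBlock is a launch pad that fires the player along its up vector when hit.
; A hit starts two timelines, with a flag blocking retriggers until the color one finishes.
; One moves the block along that axis and, at a timed event, adds a PushForce velocity impulse to player pawn 0, whatever hit it.
; The other drives red LaunchColor on the arrow's dynamic materials.
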(event `self.ReceiveBeginPlay`
  (bind _arrowhead (`self.ArrowHead`))
  (bind _arrowbody (`self.ArrowBody`))
  (bind _returnvalue (`PrimitiveComponent.CreateDynamicMaterialInstance` _arrowhead 0 (`PrimitiveComponent.GetMaterial` _arrowhead 0) "None"))
  (set `self.ArrowHeadColorMID` _returnvalue)
  (bind _returnvalue_2 (`PrimitiveComponent.CreateDynamicMaterialInstance` _arrowbody 0 (`PrimitiveComponent.GetMaterial` _arrowbody 0) "None"))
  (set `self.ArrowBodyColorMID` _returnvalue_2)
  (set `self.InitialLocation` (`self.K2_GetActorLocation`)))

(event `self.ReceiveHit`
  (params (MyComp :type "PrimitiveComponent Object Reference") (Other :type "Actor Object Reference") (OtherComp :type "PrimitiveComponent Object Reference") (bSelfMoved :type Boolean) (HitLocation :type "Vector Structure") (HitNormal :type "Vector Structure") (NormalImpulse :type "Vector Structure") (Hit :type "HitResult Structure (by ref)"))
  (bind _returnvalue (`self.GetActorUpVector`))
  (bind _pushforce (`self.PushForce`))
  (if (not (`self.bIsLaunching`))
    (set `self.bIsLaunching` true)
    (`|ExecutionSequence`
      (:`then_0`
        (bind (_direction _launchheightalpha) (`Timeline|타임라인` :!via `PlayFromStart`)
          (:`Update`
            (`self.K2_SetActorLocation` (+ (* _launchheightalpha _pushforce _returnvalue) (`self.InitialLocation`))))
          (:`LaunchTiming`
            (bind _asbp_day_0626_player (cast `/Game/Blueprints/Assignment/Day0626/BP_Day0626_Player` (`GameplayStatics.GetPlayerPawn` 0)))
            (`CharacterMovementComponent.AddImpulse` (`Character.CharacterMovement` _asbp_day_0626_player) (* _returnvalue _pushforce) true))))
      (:`then_1`
        (bind (_direction_2 _launchheightalpha_2) (`Timeline|타임라인_0` :!via `PlayFromStart`)
          (:`Update`
            (bind _returnvalue_2 (* _launchheightalpha_2 10.0))
            (`MaterialInstanceDynamic.SetVectorParameterValue` (`self.ArrowBodyColorMID`) "LaunchColor" (make `LinearColor` _returnvalue_2 0.0 0.0 1.0))
            (`MaterialInstanceDynamic.SetVectorParameterValue` (`self.ArrowHeadColorMID`) "LaunchColor" (make `LinearColor` _returnvalue_2 0.0 0.0 1.0)))
          (:`Finished`
            (set `self.bIsLaunching` false)))))))

(fn `UserConstructionScript`)