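; A block that fades away after the player touches it, then reappears after a delay.
; A Hit from player pawn 0 starts a Tick countdown that drives the Opacity parameter of the cube's dynamic material from opaque to clear.
; At zero the cube loses collision, and a second countdown restores full opacity and collision, resetting the block for reuse.
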(event `self.ReceiveBeginPlay`
  (bind _cube (`self.Cube`))
  (set `self.CurrentDisappearDuration` (`self.DisappearDuration`))
  (set `self.CurrentRegenerationDuration` (`self.RegenerationDuration`))
  (bind _returnvalue (`PrimitiveComponent.CreateDynamicMaterialInstance` _cube 0 (`PrimitiveComponent.GetMaterial` _cube 0) "None"))
  (set `self.CubeColorMID` _returnvalue))

(event `self.ReceiveHit`
  (params (MyComp :type "PrimitiveComponent Object Reference") (Other :type "Actor Object Reference") (OtherComp :type "PrimitiveComponent Object Reference") (bSelfMoved :type Boolean) (HitLocation :type "Vector Structure") (HitNormal :type "Vector Structure") (NormalImpulse :type "Vector Structure") (Hit :type "HitResult Structure (by ref)"))
  (if (== Other (`GameplayStatics.GetPlayerPawn` 0))
    (set `self.bIsDisappearing` true)))

(event `self.ReceiveTick`
  (params (DeltaSeconds :type "Float (single-precision)"))
  (if (`self.bIsDisappeared`)
    (bind _output_get (set `self.CurrentRegenerationDuration` (- (`self.CurrentRegenerationDuration`) DeltaSeconds)))
    (if (<= _output_get 0.0)
      (set `self.bIsDisappeared` false)
      (`MaterialInstanceDynamic.SetScalarParameterValue` (`self.CubeColorMID`) "Opacity" 1.0)
      (`PrimitiveComponent.SetCollisionEnabled` (`self.Cube`) "QueryAndPhysics")
      (set `self.CurrentRegenerationDuration` (`self.RegenerationDuration`)))
    (elif (`self.bIsDisappearing`)
      (bind _output_get_2 (set `self.CurrentDisappearDuration` (- (`self.CurrentDisappearDuration`) DeltaSeconds)))
      (`MaterialInstanceDynamic.SetScalarParameterValue` (`self.CubeColorMID`) "Opacity" (`KismetMathLibrary.FMax` (/ _output_get_2 (`self.DisappearDuration`))))
      (if (<= _output_get_2 0.0)
        (set `self.bIsDisappearing` false)
        (set `self.bIsDisappeared` true)
        (`PrimitiveComponent.SetCollisionEnabled` (`self.Cube`) "NoCollision")
        (set `self.CurrentDisappearDuration` (`self.DisappearDuration`))))))

(fn `UserConstructionScript`)