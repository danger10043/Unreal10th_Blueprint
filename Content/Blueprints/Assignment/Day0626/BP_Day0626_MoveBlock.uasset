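; BP_Day0626_MoveBlock is an actor that moves in an endless loop through the waypoint actors in WaypointList.
; BeginPlay snaps it to the first waypoint.
; Each Tick either advances the target with a wrapping index when within 50 units, using a squared-distance check, or steps toward it.
; Steps use SetActorLocation without sweep along the normalized direction times Velocity, with no delta time, so speed depends on frame rate.
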(event `self.ReceiveBeginPlay`
  (bind _output_get (set `self.TargetWaypoint` (`|GetArrayItem` (`self.WaypointList`))))
  (`self.K2_SetActorLocation` (`self.K2_GetActorLocation` _output_get)))

(event `self.ReceiveTick`
  (params (DeltaSeconds :type "Float (single-precision)"))
  (bind _is_close (`self.IsClose` (`self.TargetWaypoint`)))
  (if _is_close
    (`self.IncreaseIndex`)
    (set `self.TargetWaypoint` (`|GetArrayItem` (`self.WaypointList`) (`self.CurrentIndex`)))
    (else
      (`self.ApproachTarget`))))

(fn `ApproachTarget`
  (bind _returnvalue (`self.K2_GetActorLocation`))
  (`self.K2_SetActorLocation` (+ (* (`KismetMathLibrary.Normal` (- (`self.K2_GetActorLocation` (`self.TargetWaypoint`)) _returnvalue)) (`self.Velocity`)) _returnvalue)))

(fn `IncreaseIndex`
  (set `self.CurrentIndex` (mod (+ (`self.CurrentIndex`) 1) (`KismetArrayLibrary.Array_Length` (`self.WaypointList`)))))

(fn `IsClose`
  (params (`Target Waypoint` :type "/Game/Blueprints/Assignment/Day0626/BP_Day0626_MoveBlockWaypoint Object Reference"))
  (returns (`Is Close` :type Boolean))
  (return (<= (`KismetMathLibrary.Vector_DistanceSquared` (`self.K2_GetActorLocation`) (`self.K2_GetActorLocation` `Target Waypoint`)) 2500.0)))

(fn `UserConstructionScript`)