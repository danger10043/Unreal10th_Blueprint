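; BP_Day0626_Wind is a wind fan that pushes the player along its forward vector.
; Tick spins the Wings component around its roll axis at a constant rate.
; Any actor overlap sets IsPlayerFront, cleared when any overlap ends.
; While set, Tick applies a WindPower velocity-change impulse to player 0's BP_Day0626_Player movement every frame, unscaled by delta time.
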(event `self.ReceiveActorBeginOverlap`
  (params (OtherActor :type "Actor Object Reference"))
  (set `self.bIsPlayerFront` true))

(event `self.ReceiveActorEndOverlap`
  (params (OtherActor :type "Actor Object Reference"))
  (set `self.bIsPlayerFront` false))

(event `self.ReceiveTick`
  (params (DeltaSeconds :type "Float (single-precision)"))
  (bind _wings (`self.Wings`))
  (bind (_relativerotation_roll _relativerotation_pitch _relativerotation_yaw) (`KismetMathLibrary.BreakRotator` (`SceneComponent.RelativeRotation` _wings)))
  (`SceneComponent.K2_SetRelativeRotation` _wings (`KismetMathLibrary.MakeRotator` (+ (* DeltaSeconds 1080.0) _relativerotation_roll) _relativerotation_pitch _relativerotation_yaw) false false)
  (if (`self.bIsPlayerFront`)
    (bind _asbp_day_0626_player (cast `/Game/Blueprints/Assignment/Day0626/BP_Day0626_Player` (`GameplayStatics.GetPlayerPawn` 0)))
    (`CharacterMovementComponent.AddImpulse` (`Character.CharacterMovement` _asbp_day_0626_player) (* (`self.GetActorForwardVector`) (`self.WindPower`)) true)))

(fn `UserConstructionScript`)