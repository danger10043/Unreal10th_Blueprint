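; Wind effect actor that glides forward a set Distance from where it spawns, then destroys itself.
; BeginPlay creates a dynamic material on the Wind component and fixes the target point along the forward vector.
; Each Tick it steps toward the target by Velocity, without delta-time scaling, and raises Opacity from zero toward half on a distance-based curve.
; It is destroyed once within 50 units of the target.
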(event `self.ReceiveBeginPlay`
  (bind _wind (`self.Wind`))
  (bind _returnvalue (`PrimitiveComponent.CreateDynamicMaterialInstance` _wind 0 (`PrimitiveComponent.GetMaterial` _wind 0) "None"))
  (set `self.WindOpacityMID` _returnvalue)
  (set `self.TargetLocation` (+ (* (`self.GetActorForwardVector`) (`self.Distance`)) (`self.K2_GetActorLocation`))))

(event `self.ReceiveTick`
  (params (DeltaSeconds :type "Float (single-precision)"))
  (`self.ApproachTarget`)
  (`self.ApplyColor`)
  (bind _is_close (`self.IsClose`))
  (if _is_close
    (`self.K2_DestroyActor`)))

(fn `ApplyColor`
  (`MaterialInstanceDynamic.SetScalarParameterValue` (`self.WindOpacityMID`) "Opacity" (* (- 1.0 (`KismetMathLibrary.Square` (/ (`KismetMathLibrary.Vector_DistanceSquared` (`self.TargetLocation`) (`self.K2_GetActorLocation`)) (`KismetMathLibrary.Square` (`self.Distance`))))) 0.5)))

(fn `ApproachTarget`
  (bind _returnvalue (`self.K2_GetActorLocation`))
  (`self.K2_SetActorLocation` (+ (* (`KismetMathLibrary.Normal` (- (`self.TargetLocation`) _returnvalue)) (`self.Velocity`)) _returnvalue)))

(fn `IsClose`
  (returns (`Is Close` :type Boolean))
  (return (<= (`KismetMathLibrary.Vector_DistanceSquared` (`self.TargetLocation`) (`self.K2_GetActorLocation`)) 2500.0)))

(fn `UserConstructionScript`)