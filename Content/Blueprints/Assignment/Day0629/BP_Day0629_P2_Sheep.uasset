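; Sheep pawn that wanders at random and flees from nearby players, apparently to be herded into a cage.
; Looping timers drive both random AI moves and a sphere-overlap sight check, which sends the sheep directly away from a detected player.
; Each flee also tests its current position against hardcoded cage bounds, latching HasEnteredCage so later wandering picks points inside them.
; Tick draws the sight radius as a debug sphere.
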(event `self.ReceiveBeginPlay`
  (`KismetSystemLibrary.K2_SetTimerDelegate` (delegate `DetectNearbyPlayer`) (`self.SightCheckInterval`) true true)
  (`KismetSystemLibrary.K2_SetTimerDelegate` (delegate `MoveTimer`) (`self.WaitDuration`) true))

(event `MoveTimer`
  (`self.Move To Random Location`))

(event `DetectNearbyPlayer`
  (bind (_returnvalue_x _returnvalue_y) (`KismetMathLibrary.BreakVector` (`self.K2_GetActorLocation`)))
  (bind (_returnvalue_x_2 _returnvalue_y_2 _returnvalue_z) (`KismetMathLibrary.BreakVector` (`self.K2_GetActorLocation`)))
  (bind (_outactors _returnvalue) (`KismetSystemLibrary.SphereOverlapActors` (`SceneComponent.K2_GetComponentLocation` (`self.Sight`)) (`self.SightRadius`) (`|MakeArray` "ObjectTypeQuery3" :!type "EObjectTypeQuery Enum") "/Game/Blueprints/Assignment/Day0625/BP_Day0625_Player.BP_Day0625_Player_C"))
  (bind _output_get (set `self.bIsNearbyPlayer` _returnvalue))
  (if _output_get
    (bind _location (`self.GetTargetOppositeDirection` (`|GetArrayItem` _outactors)))
    (bind (_returnvalue_x_3 _returnvalue_y_3) (`KismetMathLibrary.BreakVector` (+ (`KismetMathLibrary.MakeVector` _returnvalue_x_2 _returnvalue_y_2 _returnvalue_z) (* _location (`self.RunDistance`)))))
    (bind _movementresult (`|AIMoveTo` self (`KismetMathLibrary.MakeVector` _returnvalue_x_3 _returnvalue_y_3 _returnvalue_z) null)
      (:`then`
        (bind _result (`self.IsBetween` _returnvalue_x 900.0 2700.0))
        (bind _result_2 (`self.IsBetween` _returnvalue_y -700.0 1200.0))
        (if (and _result_2 _result)
          (set `self.bHasEnteredCage` true)))
      (:`OnFail`
        (switch `EPathFollowingResult` _movementresult
          (:`Success`
            _)
          (:`Blocked`
            _)
          (:`OffPath`
            _)
          (:`Aborted`
            _)
          (:`Invalid`
            _))
        (`KismetSystemLibrary.PrintString` "Hello")))))

(event `Move To Location`
  (params (`New Location` :type "Vector Structure"))
  (`|AIMoveTo` self `New Location` null
    (:`OnSuccess`
      (if (not (`self.bIsNearbyPlayer`))
        _))))

(event `Move To Random Location`
  (bind _new_location (`self.GetRandomLocation`))
  (`self.Move To Location` _new_location))

(event `self.ReceiveTick`
  (params (DeltaSeconds :type "Float (single-precision)"))
  (`KismetSystemLibrary.DrawDebugSphere` (`SceneComponent.K2_GetComponentLocation` (`self.Sight`)) (`self.SightRadius`) 25 (struct :`R` 1.0 :`G` 1.0 :`B` 1.0 :`A` 0.6) 0.0 1.0))

(fn `GetRandomLocation`
  (returns (`New Location` :type "Vector Structure"))
  (locals (ResultLocation :type "Vector Structure"))
  (bind (_returnvalue_x _returnvalue_y _returnvalue_z) (`KismetMathLibrary.BreakVector` (`self.K2_GetActorLocation`)))
  (if (`self.bHasEnteredCage`)
    (set `local.ResultLocation` (`KismetMathLibrary.MakeVector` (`KismetMathLibrary.RandomFloatInRange` 900.0 2700.0) (`KismetMathLibrary.RandomFloatInRange` -700.0 1200.0) _returnvalue_z))
    (else
      (set `local.ResultLocation` (`NavigationSystemV1.K2_GetRandomReachablePointInRadius` (`self.K2_GetActorLocation`) (`self.RandomMoveRadius`) null null))))
  (return (`local.ResultLocation`)))

(fn `GetTargetOppositeDirection`
  (params (Target :type "Actor Object Reference"))
  (returns (Location :type "Vector Structure"))
  (return (* (`KismetMathLibrary.Normal` (- (`self.K2_GetActorLocation` Target) (`self.K2_GetActorLocation`))) -1.0)))

(fn `IsBetween`
  (params (`Target Number` :type "Float (double-precision)") (Min :type "Float (double-precision)") (Max :type "Float (double-precision)"))
  (returns (Result :type Boolean))
  (return (and (>= `Target Number` Min) (<= `Target Number` Max))))

(fn `UserConstructionScript`)