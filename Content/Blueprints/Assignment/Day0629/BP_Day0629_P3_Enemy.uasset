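; Patrolling enemy that chases the player on sight, using a three-state value for patrol, wait and chase.
; A looping timer checks sight with a sphere overlap and forward-vector angle test, without an occlusion trace.
; AI MoveTo drives chasing and the Tick-driven waypoint loop; losing sight halts it for a counted wait before resuming from the nearest waypoint.
; The state colors a debug sight cone and a Timeline-animated body material.
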(event `self.ReceiveBeginPlay`
  (bind _mesh (`self.Mesh`))
  (bind _bodycolormid (`self.BodyColorMID`))
  (`parent.ReceiveBeginPlay`)
  (`KismetSystemLibrary.K2_SetTimerDelegate` (delegate `Sight Check`) (`self.SightCheckInterval`) true)
  (bind _returnvalue (`PrimitiveComponent.CreateDynamicMaterialInstance` _mesh 0 (`PrimitiveComponent.GetMaterial` _mesh 0) "None"))
  (set `self.BodyColorMID` _returnvalue)
  (set `self.PlayerFindMaxCount` (`KismetMathLibrary.FCeil` (/ (`self.WaitDuration`) (`self.SightCheckInterval`))))
  (set `self.TargetWaypoint` (`|GetArrayItem` (`self.WaypointList`)))
  (bind (_direction _redcoloralpha) (`Timeline|타임라인` :!via `PlayFromStart`)
    (:`Update`
      (switch `int` (`self.FoundPlayerValue`)
        (:`0`
          (`MaterialInstanceDynamic.SetVectorParameterValue` _bodycolormid "Paint Tint" (make `LinearColor` 0.15 0.15 0.15 1.0)))
        (:`1`
          (`MaterialInstanceDynamic.SetVectorParameterValue` _bodycolormid "Paint Tint" (make `LinearColor` _redcoloralpha _redcoloralpha 0.0 1.0)))
        (:`2`
          (`MaterialInstanceDynamic.SetVectorParameterValue` _bodycolormid "Paint Tint" (make `LinearColor` _redcoloralpha 0.0 0.0 1.0)))))))

(event `Sight Check`
  (bind (_outactors _returnvalue) (`KismetSystemLibrary.SphereOverlapActors` (`SceneComponent.K2_GetComponentLocation` (`self.SightLocation`)) (`self.SightRadius`) (`|MakeArray` "ObjectTypeQuery3" :!type "EObjectTypeQuery Enum") "/Game/Blueprints/Assignment/Day0625/BP_Day0625_Player.BP_Day0625_Player_C"))
  (if _returnvalue
    (bind _output (`|GetArrayItem` _outactors))
    (bind _direction (`self.GetTargetDirection` _output))
    (if (<= (`KismetMathLibrary.DegAcos` (`KismetMathLibrary.Dot_VectorVector` _direction (`self.GetActorForwardVector`))) (`self.SightHalfAngle`))
      (set `self.FoundPlayerValue` 2)
      (`|AIMoveTo` self (0.0 0.0 0.0) _output
        (:`then`
          (set `self.PlayerFindCount` 0)))
      (else
        (switch `int` (`self.FoundPlayerValue`) :!label _label
          (:`1`
            (`Controller.StopMovement` (`AIBlueprintHelperLibrary.GetAIController` self))
            (`self.IncreaseCount`)
            (if (== (`self.PlayerFindMaxCount`) (`self.PlayerFindCount`))
              (set `self.FoundPlayerValue` 0)
              (set `self.PlayerFindCount` 0)
              (bind _result (`self.GetNearestWaypoint`))
              (set `self.TargetWaypoint` _result)))
          (:`2`
            (set `self.FoundPlayerValue` 1)))))
    (else
      (goto _label))))

(event `self.ReceiveTick`
  (params (DeltaSeconds :type "Float (single-precision)"))
  (bind _targetwaypoint (`self.TargetWaypoint`))
  (`parent.ReceiveTick` DeltaSeconds)
  (`self.DrawSightDebugInfo`)
  (if (== (`self.FoundPlayerValue`) 0)
    (`|AIMoveTo` self (0.0 0.0 0.0) _targetwaypoint
      (:`then`
        (bind _is_close (`self.IsClose` _targetwaypoint))
        (if _is_close
          (`self.IncreaseIndex`)
          (set `self.TargetWaypoint` (`|GetArrayItem` (`self.WaypointList`) (`self.CurrentIndex`))))))))

(fn `ApproachTarget`
  (params (`Target Waypoint` :type "/Game/Blueprints/Assignment/Day0629/BP_Day0629_P3_Waypoint Object Reference"))
  (bind _returnvalue (`KismetMathLibrary.Normal` (- (`self.K2_GetActorLocation` `Target Waypoint`) (`self.K2_GetActorLocation`))))
  (`self.K2_SetActorLocation` (+ (`self.K2_GetActorLocation`) (* _returnvalue (`self.Velocity`))))
  (`self.K2_SetActorRotation` (`KismetMathLibrary.MakeRotFromX` _returnvalue))
  (return))

(fn `DrawSightDebugInfo`
  (switch `int` (`self.FoundPlayerValue`)
    (:`0`
      (set `self.Line Color` (struct :`R` 1.0 :`G` 1.0 :`B` 1.0 :`A` 1.0)))
    (:`1`
      (set `self.Line Color` (struct :`R` 1.0 :`G` 1.0 :`A` 1.0)))
    (:`2`
      (set `self.Line Color` (struct :`R` 1.0 :`A` 1.0))))
  (`KismetSystemLibrary.DrawDebugConeInDegrees` (`SceneComponent.K2_GetComponentLocation` (`self.SightLocation`)) (`self.GetActorForwardVector`) (`self.SightRadius`) (`self.SightHalfAngle`) 0.0 20 (`self.Line Color`) 0.0 3.0))

(fn `GetNearestWaypoint`
  (returns (Result :type "/Game/Blueprints/Assignment/Day0629/BP_Day0629_P3_Waypoint Object Reference"))
  (locals (MinDistance :type "Float (double-precision)") (MinIndex :type Integer))
  (set `local.MinIndex` 0)
  (set `local.MinDistance` (`KismetMathLibrary.Vector_DistanceSquared` (`self.K2_GetActorLocation`) (`self.K2_GetActorLocation` (`|GetArrayItem` (`self.WaypointList`)))))
  (for (_array_element _array_index) (`self.WaypointList`)
    (bind _returnvalue (`KismetMathLibrary.Vector_DistanceSquared` (`self.K2_GetActorLocation`) (`self.K2_GetActorLocation` _array_element)))
    (if (< _returnvalue (`local.MinDistance`))
      (set `local.MinDistance` _returnvalue)
      (set `local.MinIndex` _array_index)))
  (return (`|GetArrayItem` (`self.WaypointList`) (`local.MinIndex`))))

(fn `GetTargetDirection`
  (params (`Direction Target` :type "Actor Object Reference"))
  (returns (Direction :type "Vector Structure"))
  (return (`KismetMathLibrary.Normal` (- (`self.K2_GetActorLocation` `Direction Target`) (`self.K2_GetActorLocation`)))))

(fn `IncreaseCount`
  (set `self.PlayerFindCount` (+ (`self.PlayerFindCount`) 1)))

(fn `IncreaseIndex`
  (set `self.CurrentIndex` (mod (+ (`self.CurrentIndex`) 1) (`KismetArrayLibrary.Array_Length` (`self.WaypointList`))))
  (return))

(fn `IsClose`
  (params (`Target Waypoint` :type "/Game/Blueprints/Assignment/Day0629/BP_Day0629_P3_Waypoint Object Reference"))
  (returns (`Is Close` :type Boolean))
  (return (<= (`KismetMathLibrary.Vector_DistanceSquared` (`self.K2_GetActorLocation` `Target Waypoint`) (`self.K2_GetActorLocation`)) 15000.0)))

(fn `UserConstructionScript`
  (`parent.UserConstructionScript`))