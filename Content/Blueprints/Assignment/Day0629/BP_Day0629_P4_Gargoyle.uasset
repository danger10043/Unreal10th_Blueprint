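; Gargoyle enemy that chases the player only while the player is moving within its sight cone.
; A looping timer runs a sphere overlap for the player, then compares the dot-product angle against the sight half-angle.
; A detected player with nonzero velocity triggers AIMoveTo, while a failed range, angle or movement check stops AI movement.
; Tick draws the sight as a flat debug cone, recolored by the found-player flag.
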(event `self.ReceiveBeginPlay`
  (`parent.ReceiveBeginPlay`)
  (`KismetSystemLibrary.K2_SetTimerDelegate` (delegate `Sight Check`) (`self.SightCheckInterval`) true))

(event `Sight Check`
  (bind (_outactors _returnvalue) (`KismetSystemLibrary.SphereOverlapActors` (`SceneComponent.K2_GetComponentLocation` (`self.SightLocation`)) (`self.SightRadius`) (`|MakeArray` "ObjectTypeQuery3" :!type "EObjectTypeQuery Enum") "/Game/Blueprints/Assignment/Day0625/BP_Day0625_Player.BP_Day0625_Player_C"))
  (if _returnvalue
    (bind _output (`|GetArrayItem` _outactors))
    (bind _direction (`self.GetTargetDirection` _output))
    (if (<= (`KismetMathLibrary.DegAcos` (`KismetMathLibrary.Dot_VectorVector` _direction (`self.GetActorForwardVector`))) (`self.SightHalfAngle`))
      (bind _asbp_day_0625_player (cast `/Game/Blueprints/Assignment/Day0625/BP_Day0625_Player` (`GameplayStatics.GetPlayerPawn` 0)))
      (if (> (`KismetMathLibrary.VSizeSquared` (`self.GetVelocity` _asbp_day_0625_player)) 0.0)
        (set `self.FoundPlayerValue` 1)
        (`|AIMoveTo` self (0.0 0.0 0.0) _output)
        (else
          (`Controller.StopMovement` (`AIBlueprintHelperLibrary.GetAIController` self) :!label _label)
          (set `self.FoundPlayerValue` 0)))
      (else
        (goto _label)))
    (else
      (goto _label))))

(event `self.ReceiveTick`
  (params (DeltaSeconds :type "Float (single-precision)"))
  (`parent.ReceiveTick` DeltaSeconds)
  (`self.DrawSightDebugInfo`))

(fn `DrawSightDebugInfo`
  (if (== (`self.FoundPlayerValue`) 1)
    (set `self.Line Color` (struct :`B` 1.0 :`A` 1.0))
    (else
      (set `self.Line Color` (struct :`R` 0.5 :`G` 0.5 :`B` 1.0 :`A` 1.0))))
  (`KismetSystemLibrary.DrawDebugConeInDegrees` (`SceneComponent.K2_GetComponentLocation` (`self.SightLocation`)) (`self.GetActorForwardVector`) (`self.SightRadius`) (`self.SightHalfAngle`) 0.0 20 (`self.Line Color`) 0.0 3.0))

(fn `GetTargetDirection`
  (params (`Direction Target` :type "Actor Object Reference"))
  (returns (Direction :type "Vector Structure"))
  (return (`KismetMathLibrary.Normal` (- (`self.K2_GetActorLocation` `Direction Target`) (`self.K2_GetActorLocation`)))))

(fn `UserConstructionScript`
  (`parent.UserConstructionScript`))