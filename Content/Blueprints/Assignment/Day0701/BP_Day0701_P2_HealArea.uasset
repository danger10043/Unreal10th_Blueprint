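; Heal area that periodically restores health to BP_Day0701_Player while its IsPlayerIn flag is set.
; A looping timer starts on BeginPlay and, every HealInterval, heals player pawn 0 by applying negative damage scaled from Heal.
; Overlap begin and end toggle the flag after casting player pawn 0, without checking OtherActor, so any overlapping actor can toggle it.
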(event `self.ReceiveBeginPlay`
  (`KismetSystemLibrary.K2_SetTimerDelegate` (delegate `ApplyDamage`) (`self.HealInterval`) true))

(event `ApplyDamage`
  (if (`self.bIsPlayerIn`)
    (bind _asbp_day_0701_player (cast `/Game/Blueprints/Assignment/Day0701/BP_Day0701_Player` (`GameplayStatics.GetPlayerPawn` 0)))
    (`GameplayStatics.ApplyDamage` _asbp_day_0701_player (* (`self.Heal`) -1.0))))

(event `self.ReceiveActorBeginOverlap`
  (params (OtherActor :type "Actor Object Reference"))
  (cast `/Game/Blueprints/Assignment/Day0701/BP_Day0701_Player` (`GameplayStatics.GetPlayerPawn` 0))
  (set `self.bIsPlayerIn` true))

(event `self.ReceiveActorEndOverlap`
  (params (OtherActor :type "Actor Object Reference"))
  (cast `/Game/Blueprints/Assignment/Day0701/BP_Day0701_Player` (`GameplayStatics.GetPlayerPawn` 0))
  (set `self.bIsPlayerIn` false))

(fn `UserConstructionScript`)