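; An EXP orb pickup that flies to the player on overlap, adds its EXP value to the player's buffer and destroys itself.
; On BeginPlay, dynamic materials and timelines animate the outer sphere's opacity and inner sphere's color, while another timeline floats the outer sphere vertically.
; The pickup timeline lerps from the outer sphere's current location, not the stored InitialLocation, toward the player's CoreLocation.
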(event `self.ReceiveBeginPlay`
  (bind _outersphere (`self.OuterSphere`))
  (bind _innersphere (`self.InnerSphere`))
  (bind _returnvalue (`PrimitiveComponent.CreateDynamicMaterialInstance` _outersphere 0 (`PrimitiveComponent.GetMaterial` _outersphere 0) "None"))
  (set `self.OuterSphereColorMID` _returnvalue)
  (bind _returnvalue_2 (`PrimitiveComponent.CreateDynamicMaterialInstance` _innersphere 0 (`PrimitiveComponent.GetMaterial` _innersphere 0) "None"))
  (set `self.InnerSphereColorMID` _returnvalue_2)
  (`self.Apply OuterSphere Color`)
  (`self.Apply InnerSphere Color`)
  (`self.Apply Sphere Vertical Move`))

(event `Apply OuterSphere Color`
  (bind _outerspherecolormid (`self.OuterSphereColorMID`))
  (`MaterialInstanceDynamic.SetVectorParameterValue` _outerspherecolormid "Color" (struct :`R` 1.0 :`G` 1.0 :`A` 1.0))
  (`MaterialInstanceDynamic.SetScalarParameterValue` _outerspherecolormid "Opacity" 0.0)
  (bind (_direction _opacitychange) (`Timeline|Outer Sphere Color Changer`)
    (:`Update`
      (`MaterialInstanceDynamic.SetScalarParameterValue` _outerspherecolormid "Opacity" _opacitychange))))

(event `Apply InnerSphere Color`
  (bind (_direction _colorchange) (`Timeline|Inner Sphere Color Changer` :!via `PlayFromStart`)
    (:`Update`
      (`MaterialInstanceDynamic.SetVectorParameterValue` (`self.InnerSphereColorMID`) "Color" (make `LinearColor` _colorchange 1.0 0.0 1.0)))))

(event `Apply Sphere Vertical Move`
  (bind (_direction _floatingalpha) (`Timeline|타임라인`)
    (:`Update`
      (`SceneComponent.K2_SetRelativeLocation` (`self.OuterSphere`) (`KismetMathLibrary.MakeVector` 0.0 0.0 (* _floatingalpha (`self.FloatingAmount`))) false false))))

(event `self.ReceiveActorBeginOverlap`
  (params (OtherActor :type "Actor Object Reference"))
  (bind _returnvalue (`GameplayStatics.GetPlayerPawn` 0))
  (if (== OtherActor _returnvalue)
    (bind _asbp_day_0701_player (cast `/Game/Blueprints/Assignment/Day0701/BP_Day0701_Player` _returnvalue))
    (set `self.InitialLocation` (`self.K2_GetActorLocation`))
    (bind (_direction _ballmovementalpha) (`Timeline|EXPBall Movement`)
      (:`Update`
        (`self.K2_SetActorLocation` (`KismetMathLibrary.VLerp` (`SceneComponent.K2_GetComponentLocation` (`self.OuterSphere`)) (`SceneComponent.K2_GetComponentLocation` (`/Game/Blueprints/Assignment/Day0701/BP_Day0701_Player.CoreLocation` _asbp_day_0701_player)) _ballmovementalpha)))
      (:`Finished`
        (`/Game/Blueprints/Assignment/Day0701/BP_Day0701_Player.Add EXPBuffer` _asbp_day_0701_player (`self.EXPValue`))
        (`self.K2_DestroyActor`)))))

(fn `UserConstructionScript`)