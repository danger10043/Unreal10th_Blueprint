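; Guard enemy that cycles through waypoints and tracks three states, apparently patrol, search and chase, shown by material tint and debug sphere color.
; FindTarget detects the player pawn with a sphere overlap plus line-of-sight trace, refilling a wait timer that Tick counts down.
; UpdateState picks the state from target and timer, playing a looking-around montage when sight is lost.
; Tick maps the state to EndColor, which a timeline lerps into the dynamic material.
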(event `self.ReceiveBeginPlay`
  (bind _mesh (`self.Mesh`))
  (`parent.ReceiveBeginPlay`)
  (bind _returnvalue (`PrimitiveComponent.CreateDynamicMaterialInstance` _mesh 0 (`PrimitiveComponent.GetMaterial` _mesh 0) "None"))
  (set `self.ColorMID` _returnvalue)
  (bind (_direction _coloralpha) (`Timeline|Color Timeline`)
    (:`Update`
      (`MaterialInstanceDynamic.SetVectorParameterValue` (`self.ColorMID`) "Paint Tint" (`KismetMathLibrary.LinearColorLerp` (`self.StartColor`) (`self.EndColor`) _coloralpha)))))

(event `self.ReceiveTick`
  (params (DeltaSeconds :type "Float (single-precision)"))
  (bind (_endcolor_r _endcolor_g _endcolor_b) (break `LinearColor` (`self.EndColor`)))
  (`parent.ReceiveTick` DeltaSeconds)
  (set `self.CurrentWaitDuration` (`KismetMathLibrary.FClamp` (- (`self.CurrentWaitDuration`) DeltaSeconds) 0.0 (`self.WaitDuration`)))
  (`KismetSystemLibrary.DrawDebugSphere` (`self.K2_GetActorLocation`) (`self.SightRadius`) 20 (make `LinearColor` _endcolor_r _endcolor_g _endcolor_b 0.2))
  (`self.Update Color` (`self.CurrentState`)))

(event `self.NextWaypoint`
  (bind _result (`/Engine/EditorBlueprintResources/StandardMacros.IncrementInt` (`self.CurrentIndex`))
    (:`  `
      (set `self.CurrentIndex` (mod _result (`KismetArrayLibrary.Array_Length` (`self.Waypoints`)))))))

(event `Update Color`
  (params (`In State` :type Integer))
  (switch `int` `In State`
    (:`0`
      (set `self.EndColor` (struct :`R` 0.15 :`G` 0.15 :`B` 0.15 :`A` 1.0)))
    (:`1`
      (set `self.EndColor` (struct :`R` 3.0 :`G` 3.0 :`A` 1.0)))
    (:`2`
      (set `self.EndColor` (struct :`R` 3.0 :`A` 1.0)))))

(event `/Game/Blueprints/Assignment/Day0702/FrameWorks/BPI_Day0702_UpdateState.UpdateState`
  (bind _out_target (`/Game/Blueprints/Practice/Test13_Day0702/BPI_Test13_FindTarget.FindTarget`))
  (`/Engine/EditorBlueprintResources/StandardMacros.IsValid` _out_target
    (:`Is Valid`
      (set `self.CurrentState` 2))
    (:`Is Not Valid`
      (if (> (`self.CurrentWaitDuration`) 0.0)
        (if (== (`self.CurrentState`) 2)
          (`|PlayMontage` (`self.Mesh`) "/Game/Blueprints/Assignment/Day0702/Animations/AM_Day0702_LookingAround.AM_Day0702_LookingAround"
            (:`then`
              _)))
        (set `self.CurrentState` 1)
        (else
          (set `self.CurrentState` 0))))))

(event `/Game/Blueprints/Assignment/Day0702/FrameWorks/BPI_Day0702_BreakDance.Break Dance`
  (`self.StopAnimMontage` "/Game/Blueprints/Assignment/Day0702/Animations/AM_Day0702_LookingAround.AM_Day0702_LookingAround"))

(fn `FindTarget`
  (returns (`Out Target` :type "Actor Object Reference"))
  (locals (ReturnTarget :type "Actor Object Reference"))
  (bind _outactors (`KismetSystemLibrary.SphereOverlapActors` (`self.K2_GetActorLocation`) (`self.SightRadius`) (`|MakeArray` "ObjectTypeQuery3" :!type "EObjectTypeQuery Enum") "/Game/Blueprints/Toy/BP_MainPlayer.BP_MainPlayer_C"))
  (for _array_element _outactors
    (if (== _array_element (`GameplayStatics.GetPlayerPawn` 0))
      (bind _outhit (`KismetSystemLibrary.LineTraceSingle` (`SceneComponent.K2_GetComponentLocation` (`self.Sight`)) (`self.K2_GetActorLocation` _array_element) "TraceTypeQuery2"))
      (if (== (`.HitActor` (`GameplayStatics.BreakHitResult` _outhit)) _array_element)
        (set `local.ReturnTarget` _array_element)
        (set `self.CurrentWaitDuration` (`self.WaitDuration`))
        (break)
        (else
          (break)))))
  (return (`local.ReturnTarget`)))

(fn `GetTargetLocation`
  (returns (`Out Location` :type "Vector Structure"))
  (bind _waypoints (`self.Waypoints`))
  (if (> (`KismetArrayLibrary.Array_Length` _waypoints) 0)
    (return (`self.K2_GetActorLocation` (`|GetArrayItem` _waypoints (`self.CurrentIndex`))))
    (else
      (return (0.0 0.0 0.0)))))

(fn `IsLookingFor`
  (returns (`Is Looking For` :type Boolean))
  (return (> (`self.CurrentWaitDuration`) 0.0)))

(fn `UserConstructionScript`
  (`parent.UserConstructionScript`))