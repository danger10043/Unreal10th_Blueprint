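; BP_Day0617_P2 is an actor that patrols a looping path of waypoint positions.
; On BeginPlay it snaps to the first point, then each Tick steps toward the target along a normalized direction scaled by MoveSpeed, without delta time or sweep.
; When the squared distance to the target falls within a small threshold, the target index advances with modulo wraparound.
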(event `self.ReceiveBeginPlay`
  (`self.K2_SetActorLocation` (`|GetArrayItem` (`self.WayPointList`))))

(event `self.ReceiveTick`
  (params (DeltaSeconds :type "Float (single-precision)"))
  (bind _output (`|GetArrayItem` (`self.WayPointList`) (`self.TargetWayPointIndex`)))
  (if (<= (`KismetMathLibrary.Vector_DistanceSquared` (`self.K2_GetActorLocation`) _output) 50.0)
    (set `self.TargetWayPointIndex` (mod (+ (`self.TargetWayPointIndex`) 1) (`KismetArrayLibrary.Array_Length` (`self.WayPointList`))))
    (else
      (`self.K2_SetActorLocation` (+ (* (`self.MoveSpeed`) (`KismetMathLibrary.Normal` (- _output (`self.K2_GetActorLocation`)))) (`self.K2_GetActorLocation`))))))

(fn `UserConstructionScript`)