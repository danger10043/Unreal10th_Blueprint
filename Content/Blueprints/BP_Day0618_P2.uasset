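; BP_Day0618_P2 is an actor with a propeller component that homes in on the first player's pawn.
; Each Tick it rotates to face the pawn and steps toward it by MoveSpeed, with no delta-time scaling or collision sweep.
; The same Tick spins PlanePropeller by adding RotateSpeed to its relative roll, also per frame.
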(event `self.ReceiveTick`
  (params (DeltaSeconds :type "Float (single-precision)"))
  (bind _returnvalue (`self.K2_GetActorLocation`))
  (bind _planepropeller (`self.PlanePropeller`))
  (bind (_relativerotation_roll _relativerotation_pitch _relativerotation_yaw) (`KismetMathLibrary.BreakRotator` (`SceneComponent.RelativeRotation` _planepropeller)))
  (bind _output_get (set `self.TargetLocation` (`self.K2_GetActorLocation` (`GameplayStatics.GetPlayerPawn` 0))))
  (set `self.TargetDirection` (`KismetMathLibrary.Normal` (- _output_get _returnvalue)))
  (`self.K2_SetActorRotation` (`KismetMathLibrary.Conv_VectorToRotator` (`self.TargetDirection`)))
  (`self.K2_SetActorLocation` (+ (* (`self.TargetDirection`) (`self.MoveSpeed`)) (+ (0.0 0.0 0.0) _returnvalue)))
  (`SceneComponent.K2_SetRelativeRotation` _planepropeller (`KismetMathLibrary.MakeRotator` (+ (`self.RotateSpeed`) _relativerotation_roll) _relativerotation_pitch _relativerotation_yaw) false false))

(fn `UserConstructionScript`)