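; Test projectile actor that homes in on the player character's mesh through its ProjectileMovement component.
; Each tick it turns to face the Scene component's velocity.
; It also increments a counter each tick and attaches a new, scaled-down tutorial particle emitter to its Niagara component until the counter passes ParticleCount.
; Despite the collision-test name, the overlap event has no logic.
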(event `self.ReceiveBeginPlay`
  (set `ProjectileMovementComponent.HomingTargetComponent` (`Character.Mesh` (`GameplayStatics.GetPlayerCharacter` 0)) (`self.ProjectileMovement`)))

(event `self.ReceiveActorBeginOverlap`
  (params (OtherActor :type "Actor Object Reference")))

(event `self.ReceiveTick`
  (params (DeltaSeconds :type "Float (single-precision)"))
  (set `self.CurrentParticleCount` (+ (`self.CurrentParticleCount`) 1))
  (`self.K2_SetActorRotation` (`KismetMathLibrary.Conv_VectorToRotator` (`SceneComponent.GetComponentVelocity` (`self.Scene`))))
  (if (<= (`self.CurrentParticleCount`) (`self.ParticleCount`))
    (`GameplayStatics.SpawnEmitterAttached` "/Engine/Tutorial/SubEditors/TutorialAssets/TutorialParticleSystem.TutorialParticleSystem" (`self.Niagara`) "None" (0.0 0.0 0.0) (struct) (0.3 0.3 0.0))))

(fn `UserConstructionScript`)