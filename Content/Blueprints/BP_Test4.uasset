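; BP_Test4 is a test actor that sets up a throw from the player's position when the player pawn rises above a height threshold.
; On Tick, the first frame above the threshold teleports the actor to the pawn, stores the pawn's forward vector and sets HasThrown.
; Dropping back to or below the threshold clears the flag.
; The logic that would move the actor along that direction by Speed is disconnected, so it never runs.
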(event `self.ReceiveTick`
  (params (DeltaSeconds :type "Float (single-precision)"))
  (bind _returnvalue (`GameplayStatics.GetPlayerPawn` 0))
  (bind (_returnvalue_x _returnvalue_y _returnvalue_z) (`KismetMathLibrary.BreakVector` (`self.K2_GetActorLocation` (`GameplayStatics.GetPlayerPawn` 0))))
  (if (> _returnvalue_z 100.0)
    (if (not (`self.bHasThrown`))
      (`self.K2_SetActorLocation` (`self.K2_GetActorLocation` _returnvalue))
      (set `self.Direction` (`self.GetActorForwardVector` _returnvalue))
      (set `self.bHasThrown` true))
    (else
      (set `self.bHasThrown` false))))

(fn `UserConstructionScript`)