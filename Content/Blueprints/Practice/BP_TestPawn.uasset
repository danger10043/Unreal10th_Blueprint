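; Practice pawn that the player moves on the horizontal plane with Enhanced Input, with a hold-to-boost action.
; Movement input becomes a normalized world direction, scaled by move speed and a boost multiplier.
; Starting and releasing boost change the multiplier and play separate timelines that animate spring arm length.
; Tick turns the actor along player 0 pawn's velocity; the fire input is an empty stub.
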(event `self.ReceiveBeginPlay`
  (`EnhancedInputSubsystemInterface.AddMappingContext` (subsystem `EnhancedInputLocalPlayerSubsystem`) "/Game/Blueprints/FrameWork/Input/IMC_TestPawn.IMC_TestPawn" 0 (struct))
  (set `self.SpeedMultipleValue` 1.0))

(event `EnhancedInput|/Game/Blueprints/FrameWork/Input/IA_Test1_FireAction`
  (params (ActionValue :type Boolean) (ElapsedSeconds :type "Float (double-precision)") (TriggeredSeconds :type "Float (double-precision)") (InputAction :type "InputAction Object Reference" :default "/Game/Blueprints/FrameWork/Input/IA_Test1_FireAction.IA_Test1_FireAction")))

(event `EnhancedInput|/Game/Blueprints/FrameWork/Input/IA_Test1_Movement`
  (params (ActionValue :type "Vector2D Structure") (ElapsedSeconds :type "Float (double-precision)") (TriggeredSeconds :type "Float (double-precision)") (InputAction :type "InputAction Object Reference" :default "/Game/Blueprints/FrameWork/Input/IA_Test1_Movement.IA_Test1_Movement"))
  (:`Triggered`
    (bind _output_get (set `self.MoveDirection` (`KismetMathLibrary.Normal` (`KismetMathLibrary.MakeVector` ActionValue_Y ActionValue_X))))
    (`self.AddMovementInput` _output_get (* (`self.MoveSpeed`) (`self.SpeedMultipleValue`))))
  (:`Completed`
    (set `self.MoveDirection` (0.0 0.0 0.0))))

(event `EnhancedInput|/Game/Blueprints/FrameWork/Input/IA_Test1_Boost`
  (params (ActionValue :type Boolean) (ElapsedSeconds :type "Float (double-precision)") (TriggeredSeconds :type "Float (double-precision)") (InputAction :type "InputAction Object Reference" :default "/Game/Blueprints/FrameWork/Input/IA_Test1_Boost.IA_Test1_Boost"))
  (bind _springarm (`self.SpringArm`))
  (:`Started`
    (set `self.SpeedMultipleValue` 4.0)
    (bind (_direction _camaramoving) (`Timeline|타임라인` :!via `PlayFromStart`)
      (:`Update`
        (set `SpringArmComponent.TargetArmLength` _camaramoving _springarm))))
  (:`Completed`
    (set `self.SpeedMultipleValue` 1.0)
    (bind (_direction_2 _camaramoving_2) (`Timeline|타임라인_0` :!via `PlayFromStart`)
      (:`Update`
        (set `SpringArmComponent.TargetArmLength` _camaramoving_2 _springarm)))))

(event `self.ReceiveTick`
  (params (DeltaSeconds :type "Float (single-precision)"))
  (`self.K2_SetActorRotation` (`KismetMathLibrary.Conv_VectorToRotator` (`self.GetVelocity` (`GameplayStatics.GetPlayerPawn` 0)))))

(fn `UserConstructionScript`)