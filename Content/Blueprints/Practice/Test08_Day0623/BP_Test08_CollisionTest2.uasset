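; Practice collision-test projectile that homes on the player character's mesh and knocks the player back on impact.
; BeginPlay sets the homing target, and Tick rotates the actor to face its Scene component's velocity.
; Tick also attaches one tutorial particle emitter per frame to the Niagara component until ParticleCount is reached.
; Hitting the player applies a large velocity-change impulse along the inverted hit normal via BP_Day0622_Player's CharacterMovement.
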(event `self.ReceiveBeginPlay`
  (set `ProjectileMovementComponent.HomingTargetComponent` (`Character.Mesh` (`GameplayStatics.GetPlayerCharacter` 0)) (`self.ProjectileMovement`)))

(event `self.ReceiveActorBeginOverlap`
  (params (OtherActor :type "Actor Object Reference")))

(event `self.ReceiveTick`
  (params (DeltaSeconds :type "Float (single-precision)"))
  (set `self.CurrentParticleCount` (+ (`self.CurrentParticleCount`) 1))
  (`self.K2_SetActorRotation` (`KismetMathLibrary.Conv_VectorToRotator` (`SceneComponent.GetComponentVelocity` (`self.Scene`))))
  (if (<= (`self.CurrentParticleCount`) (`self.ParticleCount`))
    (`GameplayStatics.SpawnEmitterAttached` "/Engine/Tutorial/SubEditors/TutorialAssets/TutorialParticleSystem.TutorialParticleSystem" (`self.Niagara`) "None" (0.0 0.0 0.0) (struct) (0.3 0.3 0.0))))

(event `self.ReceiveHit`
  (params (MyComp :type "PrimitiveComponent Object Reference") (Other :type "Actor Object Reference") (OtherComp :type "PrimitiveComponent Object Reference") (bSelfMoved :type Boolean) (HitLocation :type "Vector Structure") (HitNormal :type "Vector Structure") (NormalImpulse :type "Vector Structure") (Hit :type "HitResult Structure (by ref)"))
  (bind _returnvalue (`GameplayStatics.GetPlayerPawn` 0))
  (if (== Other _returnvalue)
    (bind _asbp_day_0622_player (cast `/Game/Blueprints/Assignment/Day0622/BP_Day0622_Player` _returnvalue))
    (`CharacterMovementComponent.AddImpulse` (`Character.CharacterMovement` _asbp_day_0622_player) (* HitNormal 10000.0 -1.0) true)))

(fn `UserConstructionScript`)