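; BP_Test08_P2 is a sliding double door that opens on actor overlap and closes when the overlap ends.
; It stores both doors' initial relative locations on BeginPlay, then a timeline offsets them in opposite directions along Y, reversing to close.
; Open, Close and SwitchOpenState events share the same paths, each of which flips the Opened flag and restarts the timeline from one end.
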(event `self.ReceiveBeginPlay`
  (set `self.LeftDoorInitialLocation` (`SceneComponent.RelativeLocation` (`self.LeftDoor`)))
  (set `self.RightDoorInitialLocation` (`SceneComponent.RelativeLocation` (`self.RightDoor`))))

(event `self.ReceiveActorBeginOverlap`
  (params (OtherActor :type "Actor Object Reference"))
  (bind (_leftdoorinitiallocation_x _leftdoorinitiallocation_y _leftdoorinitiallocation_z) (`KismetMathLibrary.BreakVector` (`self.LeftDoorInitialLocation`)))
  (bind (_rightdoorinitiallocation_x _rightdoorinitiallocation_y _rightdoorinitiallocation_z) (`KismetMathLibrary.BreakVector` (`self.RightDoorInitialLocation`)))
  (`self.SwitchBOpened` :!label _label)
  (bind (_direction _doormovement) (`Timeline|타임라인` :!via `PlayFromStart` :!label _label_2)
    (:`Update`
      (bind _returnvalue (* _doormovement 85.0))
      (`SceneComponent.K2_SetRelativeLocation` (`self.LeftDoor`) (`KismetMathLibrary.MakeVector` _leftdoorinitiallocation_x (+ _leftdoorinitiallocation_y _returnvalue) _leftdoorinitiallocation_z) false false)
      (`SceneComponent.K2_SetRelativeLocation` (`self.RightDoor`) (`KismetMathLibrary.MakeVector` _rightdoorinitiallocation_x (+ _rightdoorinitiallocation_y (* -1.0 _returnvalue)) _rightdoorinitiallocation_z) false false))))

(event `Open`
  (goto _label))

(event `Close`
  (`self.SwitchBOpened` :!label _label_3)
  (goto _label_2 :!via `ReverseFromEnd`))

(event `self.ReceiveActorEndOverlap`
  (params (OtherActor :type "Actor Object Reference"))
  (goto _label_3))

(event `Switch Open State`
  (if (`self.bOpened`)
    (goto _label_3)
    (else
      (goto _label))))

(event `self.ReceiveTick`
  (params (DeltaSeconds :type "Float (single-precision)")))

(fn `SwitchBOpened`
  (set `self.bOpened` (not (`self.bOpened`)))
  (return))

(fn `UserConstructionScript`)