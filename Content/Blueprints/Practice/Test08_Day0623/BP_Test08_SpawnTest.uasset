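; BP_Test08_SpawnTest is a practice trigger actor that spawns a configurable actor when the player pawn overlaps it.
; On overlap with player pawn 0, it calls a SpawnItem event that spawns the SpawnTarget class at the SpawnTransform component's world transform.
; If SpawnTarget is not set, it prints a red warning instead.
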(event `self.ReceiveActorBeginOverlap`
  (params (OtherActor :type "Actor Object Reference"))
  (if (== OtherActor (`GameplayStatics.GetPlayerPawn` 0))
    (`self.SpawnItem`)))

(event `self.ReceiveActorEndOverlap`
  (params (OtherActor :type "Actor Object Reference")))

(event `SpawnItem`
  (bind _spawntarget (`self.SpawnTarget`))
  (if (`KismetSystemLibrary.IsValidClass` _spawntarget)
    (`|SpawnActorFromClass` _spawntarget (`SceneComponent.K2_GetComponentToWorld` (`self.SpawnTransform`)) "Undefined" "MultiplyWithRoot" null null)
    (else
      (`KismetSystemLibrary.PrintString` "SpawnTarge이 없습니다." true true (struct :`R` 1.0 :`A` 1.0)))))

(fn `UserConstructionScript`)