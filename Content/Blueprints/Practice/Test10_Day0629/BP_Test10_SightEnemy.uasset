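; BP_Test10_SightEnemy is a practice enemy that spots the player inside a forward vision cone and chases it with AI MoveTo.
; A looping timer runs a sphere overlap for the player pawn, then compares the angle to its forward vector against a half-angle; failure stops movement.
; The found flag drives a Timeline-animated red tint on a dynamic body material and the color of a debug cone drawn each Tick.
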(event `self.ReceiveBeginPlay`
  (bind _mesh (`self.Mesh`))
  (bind _bodycolormid (`self.BodyColorMID`))
  (`parent.ReceiveBeginPlay`)
  (`KismetSystemLibrary.K2_SetTimerDelegate` (delegate `Sight Check`) (`self.SightCheckInterval`) true)
  (bind _returnvalue (`PrimitiveComponent.CreateDynamicMaterialInstance` _mesh 0 (`PrimitiveComponent.GetMaterial` _mesh 0) "None"))
  (set `self.BodyColorMID` _returnvalue)
  (bind (_direction _redcoloralpha) (`Timeline|타임라인` :!via `PlayFromStart`)
    (:`Update`
      (if (== (`self.FoundPlayerValue`) 1)
        (`MaterialInstanceDynamic.SetVectorParameterValue` _bodycolormid "Paint Tint" (make `LinearColor` _redcoloralpha 0.15 0.15 1.0))
        (else
          (`MaterialInstanceDynamic.SetVectorParameterValue` _bodycolormid "Paint Tint" (make `LinearColor` 0.15 0.15 0.15 1.0)))))))

(event `Sight Check`
  (bind (_outactors _returnvalue) (`KismetSystemLibrary.SphereOverlapActors` (`SceneComponent.K2_GetComponentLocation` (`self.SightLocation`)) (`self.SightRadius`) (`|MakeArray` "ObjectTypeQuery3" :!type "EObjectTypeQuery Enum") "/Game/Blueprints/Assignment/Day0625/BP_Day0625_Player.BP_Day0625_Player_C"))
  (if _returnvalue
    (bind _output (`|GetArrayItem` _outactors))
    (bind _direction (`self.GetTargetDirection` _output))
    (if (<= (`KismetMathLibrary.DegAcos` (`KismetMathLibrary.Dot_VectorVector` _direction (`self.GetActorForwardVector`))) (`self.SightHalfAngle`))
      (set `self.FoundPlayerValue` 1)
      (`|AIMoveTo` self (0.0 0.0 0.0) _output)
      (else
        (`Controller.StopMovement` (`AIBlueprintHelperLibrary.GetAIController` self) :!label _label)
        (set `self.FoundPlayerValue` 0)))
    (else
      (goto _label))))

(event `self.ReceiveTick`
  (params (DeltaSeconds :type "Float (single-precision)"))
  (`parent.ReceiveTick` DeltaSeconds)
  (`self.DrawSightDebugInfo`))

(fn `DrawSightDebugInfo`
  (if (== (`self.FoundPlayerValue`) 1)
    (set `self.Line Color` (struct :`R` 1.0 :`A` 1.0))
    (else
      (set `self.Line Color` (struct :`R` 1.0 :`G` 1.0 :`B` 1.0 :`A` 1.0))))
  (`KismetSystemLibrary.DrawDebugConeInDegrees` (`SceneComponent.K2_GetComponentLocation` (`self.SightLocation`)) (`self.GetActorForwardVector`) (`self.SightRadius`) (`self.SightHalfAngle`) 0.0 20 (`self.Line Color`) 0.0 3.0))

(fn `GetTargetDirection`
  (params (`Direction Target` :type "Actor Object Reference"))
  (returns (Direction :type "Vector Structure"))
  (return (`KismetMathLibrary.Normal` (- (`self.K2_GetActorLocation` `Direction Target`) (`self.K2_GetActorLocation`)))))

(fn `UserConstructionScript`
  (`parent.UserConstructionScript`))