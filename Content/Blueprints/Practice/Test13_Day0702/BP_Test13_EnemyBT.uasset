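; Practice enemy Blueprint that supplies waypoint patrol data, apparently for a Behavior Tree given its name.
; GetTargetLocation returns the location of the waypoint actor at CurrentIndex, or the zero vector when the Waypoints array is empty.
; The NextWaypoint event increments CurrentIndex and wraps it by the array length to loop the route, without an empty-array check.
; It contains no movement logic, and BeginPlay, overlap and Tick are disabled stubs.
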(event `/Game/Blueprints/Practice/Test13_Day0702/BPI_Test13_WaypointUser.NextWaypoint`
  (bind _result (`/Engine/EditorBlueprintResources/StandardMacros.IncrementInt` (`self.CurrentIndex`))
    (:`  `
      (set `self.CurrentIndex` (mod _result (`KismetArrayLibrary.Array_Length` (`self.Waypoints`)))))))

(fn `GetTargetLocation`
  (returns (`Out Location` :type "Vector Structure"))
  (bind _waypoints (`self.Waypoints`))
  (if (> (`KismetArrayLibrary.Array_Length` _waypoints) 0)
    (return (`self.K2_GetActorLocation` (`|GetArrayItem` _waypoints (`self.CurrentIndex`))))
    (else
      (return (0.0 0.0 0.0)))))

(fn `UserConstructionScript`
  (`parent.UserConstructionScript`))