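; Practice enemy Blueprint (EnemyBT3) that provides sight-based player detection and looping waypoint patrol data, with no movement logic of its own.
; FindTarget overlaps a SightRadius sphere for the player pawn, then returns it only if a Camera-channel trace from the Sight component hits it first.
; GetTargetLocation returns the current waypoint's position, and NextWaypoint advances the index with wraparound.
; Tick draws the sight sphere for debugging.
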(event `self.ReceiveTick`
  (params (DeltaSeconds :type "Float (single-precision)"))
  (`parent.ReceiveTick` DeltaSeconds)
  (`KismetSystemLibrary.DrawDebugSphere` (`self.K2_GetActorLocation`) (`self.SightRadius`) 20 (struct :`R` 1.0 :`G` 1.0 :`B` 1.0 :`A` 0.6)))

(event `/Game/Blueprints/Practice/Test13_Day0702/BPI_Test13_WaypointUser.NextWaypoint`
  (bind _result (`/Engine/EditorBlueprintResources/StandardMacros.IncrementInt` (`self.CurrentIndex`))
    (:`  `
      (set `self.CurrentIndex` (mod _result (`KismetArrayLibrary.Array_Length` (`self.Waypoints`)))))))

(fn `FindTarget`
  (returns (`Out Target` :type "Actor Object Reference"))
  (locals (ReturnTarget :type "Actor Object Reference"))
  (bind _outactors (`KismetSystemLibrary.SphereOverlapActors` (`self.K2_GetActorLocation`) (`self.SightRadius`) (`|MakeArray` "ObjectTypeQuery3" :!type "EObjectTypeQuery Enum") "/Game/Blueprints/Toy/BP_MainPlayer.BP_MainPlayer_C"))
  (for _array_element _outactors
    (if (== _array_element (`GameplayStatics.GetPlayerPawn` 0))
      (bind _outhit (`KismetSystemLibrary.LineTraceSingle` :`Start` (`SceneComponent.K2_GetComponentLocation` (`self.Sight`)) :`End` (`self.K2_GetActorLocation` _array_element) :`TraceChannel` "TraceTypeQuery2" :`DrawDebugType` "ForOneFrame"))
      (if (== (`.HitActor` (`GameplayStatics.BreakHitResult` _outhit)) _array_element)
        (set `local.ReturnTarget` _array_element)
        (break)
        (else
          (break)))))
  (return (`local.ReturnTarget`)))

(fn `GetTargetLocation`
  (returns (`Out Location` :type "Vector Structure"))
  (bind _waypoints (`self.Waypoints`))
  (if (> (`KismetArrayLibrary.Array_Length` _waypoints) 0)
    (return (`self.K2_GetActorLocation` (`|GetArrayItem` _waypoints (`self.CurrentIndex`))))
    (else
      (return (0.0 0.0 0.0)))))

(fn `UserConstructionScript`
  (`parent.UserConstructionScript`))