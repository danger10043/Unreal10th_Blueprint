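; BP_Toy1 is a toy actor that follows player pawn 0 and changes its pose with the pawn's movement.
; Every Tick checks the pawn's speed: when nearly stationary, the toy shrinks to half scale and hovers above and behind the pawn at a fixed rotation.
; While the pawn moves, the toy returns to full scale at the pawn's location, levels its pitch and spins in yaw by speed times RotateSpeed per frame, without delta-time scaling.
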(event `self.ReceiveBeginPlay`)

(event `self.ReceiveTick`
  (params (DeltaSeconds :type "Float (single-precision)"))
  (bind _returnvalue (`GameplayStatics.GetPlayerPawn` 0))
  (bind (_returnvalue_roll _returnvalue_pitch _returnvalue_yaw) (`KismetMathLibrary.BreakRotator` (`self.K2_GetActorRotation`)))
  (bind _returnvalue_2 (`GameplayStatics.GetPlayerPawn` 0))
  (bind (_returnvalue_x _returnvalue_y _returnvalue_z) (`KismetMathLibrary.BreakVector` (+ (`self.K2_GetActorLocation` _returnvalue_2) (* (`self.GetActorForwardVector` _returnvalue_2) -80.0))))
  (if (< (`KismetMathLibrary.VSize` (`self.GetVelocity` (`GameplayStatics.GetPlayerPawn` 0))) 0.03)
    (`self.K2_SetActorRotation` (struct :`Pitch` 270.0))
    (`self.K2_SetActorLocation` (`KismetMathLibrary.MakeVector` _returnvalue_x _returnvalue_y (+ _returnvalue_z 250.0)))
    (`self.SetActorScale3D` (0.5 0.5 0.5))
    (else
      (`self.SetActorScale3D` (1.0 1.0 1.0))
      (`self.K2_SetActorRotation` (`KismetMathLibrary.MakeRotator` _returnvalue_roll 0.0 _returnvalue_yaw))
      (`self.K2_SetActorRotation` (`KismetMathLibrary.MakeRotator` _returnvalue_roll _returnvalue_pitch (+ _returnvalue_yaw (* (`KismetMathLibrary.VSize` (`self.GetVelocity` _returnvalue)) (`self.RotateSpeed`)))))
      (`self.K2_SetActorLocation` (`self.K2_GetActorLocation` _returnvalue)))))

(fn `UserConstructionScript`)