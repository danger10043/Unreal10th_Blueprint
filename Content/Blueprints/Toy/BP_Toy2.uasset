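; BP_Toy2 is a sword toy that swings around the player when they jump, then settles at their side.
; Tick treats player height above a fixed world Z as a jump, starting a timeline that sweeps the sword through a sine/cosine half-circle in front while pitching it.
; Once the player is back below that height, a second timeline lerps it beside them.
; SwordState sequences swing, return and follow, which re-arms the attack.
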(event `self.ReceiveBeginPlay`
  (set `self.bHasJumped` false)
  (set `self.SwordState` 0))

(event `self.ReceiveTick`
  (params (DeltaSeconds :type "Float (single-precision)"))
  (bind _returnvalue (`GameplayStatics.GetPlayerPawn` 0))
  (bind _returnvalue_2 (`GameplayStatics.GetPlayerPawn` 0))
  (bind _returnvalue_3 (`GameplayStatics.GetPlayerPawn` 0))
  (bind (_initialrotate_roll _initialrotate_pitch _initialrotate_yaw) (`KismetMathLibrary.BreakRotator` (`self.InitialRotate`)))
  (bind (_returnvalue_x _returnvalue_y _returnvalue_z) (`KismetMathLibrary.BreakVector` (`self.K2_GetActorLocation` _returnvalue_3)))
  (bind (_returnvalue_x_2 _returnvalue_y_2 _returnvalue_z_2) (`KismetMathLibrary.BreakVector` (`self.K2_GetActorLocation` _returnvalue)))
  (bind (_returnvalue_roll _returnvalue_pitch _returnvalue_yaw) (`KismetMathLibrary.BreakRotator` (`self.K2_GetActorRotation` _returnvalue)))
  (bind (_returnvalue_roll_2 _returnvalue_pitch_2 _returnvalue_yaw_2) (`KismetMathLibrary.BreakRotator` (`self.K2_GetActorRotation` _returnvalue_3)))
  (bind (_returnvalue_x_3 _returnvalue_y_3 _returnvalue_z_3) (`KismetMathLibrary.BreakVector` (`self.K2_GetActorLocation` _returnvalue)))
  (bind (_returnvalue_roll_3 _returnvalue_pitch_3 _returnvalue_yaw_3) (`KismetMathLibrary.BreakRotator` (`self.K2_GetActorRotation` _returnvalue_2)))
  (if (> _returnvalue_z 100.0)
    (if (not (`self.bHasJumped`))
      (`KismetSystemLibrary.PrintString` "Hello")
      (set `self.bHasJumped` true)
      (set `self.InitialRotate` (`self.K2_GetActorRotation`))
      (`self.K2_SetActorRotation` (`KismetMathLibrary.MakeRotator` (+ _returnvalue_roll 90.0) (+ _returnvalue_pitch 270.0) _returnvalue_yaw))
      (`self.K2_SetActorLocation` (`KismetMathLibrary.MakeVector` _returnvalue_x_2 _returnvalue_y_2 (+ _returnvalue_z_2 150.0)))
      (bind (_direction _swordmovementalpha) (`Timeline|타임라인` :!via `PlayFromStart`)
        (:`Update`
          (`self.K2_SetActorRotation` (`KismetMathLibrary.MakeRotator` _initialrotate_roll (+ (+ (* _swordmovementalpha -180.0) 270.0) _initialrotate_pitch) _initialrotate_yaw))
          (bind _returnvalue_4 (`KismetMathLibrary.MultiplyByPi` _swordmovementalpha))
          (bind (_returnvalue_x_4 _returnvalue_y_4) (`KismetMathLibrary.BreakVector` (* (`KismetMathLibrary.Sin` _returnvalue_4) 150.0 (`self.GetActorForwardVector` _returnvalue))))
          (`self.K2_SetActorLocation` (`KismetMathLibrary.MakeVector` (+ _returnvalue_x_4 _returnvalue_x_3) (+ _returnvalue_y_4 _returnvalue_y_3) (+ _returnvalue_z_3 (* (`KismetMathLibrary.Cos` _returnvalue_4) -150.0)))))
        (:`Finished`
          (set `self.SwordState` 1))))
    (elif (== (`self.SwordState`) 1)
      (set `self.SwordState` 2)
      (set `self.InitialLocationAfterAttack` (`self.K2_GetActorLocation`))
      (set `self.InitialRotationAfterAttack` (`self.K2_GetActorRotation`))
      (bind (_direction_2 _swordmovementalpha_2) (`Timeline|타임라인_0` :!via `PlayFromStart`)
        (:`Update`
          (`self.K2_SetActorLocation` (`KismetMathLibrary.VLerp` (`self.InitialLocationAfterAttack`) (+ (`self.K2_GetActorLocation` _returnvalue_2) (* (`KismetMathLibrary.RotateAngleAxis` (`self.GetActorForwardVector` _returnvalue_2) 90.0 (0.0 0.0 1.0)) 80.0)) _swordmovementalpha_2))
          (`self.K2_SetActorRotation` (`KismetMathLibrary.RLerp` (`self.InitialRotationAfterAttack`) (`KismetMathLibrary.MakeRotator` _returnvalue_roll_3 (+ _returnvalue_pitch_3 180.0) _returnvalue_yaw_3) _swordmovementalpha_2)))
        (:`Finished`
          (set `self.SwordState` 3)))
      (elif (== (`self.SwordState`) 3)
        (`self.K2_SetActorRotation` (`KismetMathLibrary.MakeRotator` _returnvalue_roll_2 (+ _returnvalue_pitch_2 180.0) _returnvalue_yaw_2))
        (`self.K2_SetActorLocation` (+ (`self.K2_GetActorLocation` _returnvalue_3) (* (`KismetMathLibrary.RotateAngleAxis` (`self.GetActorForwardVector` _returnvalue_3) 90.0 (0.0 0.0 1.0)) 80.0)))
        (set `self.bHasJumped` false)))))

(fn `UserConstructionScript`)